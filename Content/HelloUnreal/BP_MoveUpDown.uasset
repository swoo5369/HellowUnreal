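; BP_MoveUpDown is an actor whose Cube component oscillates vertically between relative height zero and the EndUp limit.
; Each Tick shifts the cube by a fixed relative offset in the direction set by IsMoveUp, flipping that flag when a bound is reached.
; Movement is not scaled by delta time, so speed depends on frame rate, and it runs without sweep.
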(event EventTick
  (params (DeltaSeconds :type Float%20%28single-precision%29))
  (bind _cube (Variables|Default|GetCube))
  (bind _cube_2 (Variables|Default|GetCube))
  (if (Variables|Default|GetIsMoveUp)
    (Transformation|AddRelativeLocation _cube_2 "0, 0,10.000000" false false)
    (if (>= (.z (Variables|/Script/Engine.SceneComponent|GetRelativeLocation _cube_2)) (Variables|Default|GetEndUp))
      (Variables|Default|SetIsMoveUp false))
    (else
      (Transformation|AddRelativeLocation _cube "0, 0,-10.000000" false false)
      (if (< (.z (Variables|/Script/Engine.SceneComponent|GetRelativeLocation _cube)) 0.0)
        (Variables|Default|SetIsMoveUp true)))))

(fn ConstructionScript)