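; BP_TimeLineMove1 is a timeline movement Blueprint that slides a Sphere along straight edges of a square-like path in relative space.
; BeginPlay switches on MoveType; the Up, Left and Down timelines each drive SetRelativeLocation, scaled by EndPoint with hardcoded offsets.
; Each Finished event advances MoveType and re-enters the switch, forming a chained state machine.
; Right has no connected branch, so movement stops there; its apparent timeline and the reset to Up are unwired.
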(event EventBeginPlay
  (switch Utilities|FlowControl|Switch|SwitchonEn_MoveType (Variables|Default|GetMoveType) :!label _label
    (:NewEnumerator0)
    (:NewEnumerator1
      (bind _value (Timeline|타임라인_1 Play)
        (:Update
          (Transformation|SetRelativeLocation (Variables|Default|GetSphere) (Math|Vector|MakeVector 5e+02 (* (Variables|Default|GetEndPoint) (* _value -1.0)) 0.0) false false))
        (:Finished
          (Variables|Default|SetMoveType "NewEnumerator2")
          (goto _label))))
    (:NewEnumerator2
      (bind _value_2 (Timeline|타임라인_2 Play)
        (:Update
          (Transformation|SetRelativeLocation (Variables|Default|GetSphere) (Math|Vector|MakeVector (- 5e+02 (* (Variables|Default|GetEndPoint) _value_2)) -5e+02 0.0) false false))
        (:Finished
          (Variables|Default|SetMoveType "NewEnumerator3")
          (goto _label))))
    (:NewEnumerator3
      (bind _value_3 (Timeline|타임라인_3 Play)
        (:Update
          (Transformation|SetRelativeLocation (Variables|Default|GetSphere) (Math|Vector|MakeVector 0.0 (+ (* (Variables|Default|GetEndPoint) _value_3) -5e+02) 0.0) false false))
        (:Finished
          (Variables|Default|SetMoveType "NewEnumerator0")
          (goto _label))))))

(fn ConstructionScript)